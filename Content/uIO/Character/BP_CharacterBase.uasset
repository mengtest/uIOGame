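; Base character with a sprite body, health bar widget, attacking and death drop.
; Damage feeds BPCState as a negative change, while LookAt turns the sprite by yaw toward a target.
; Attack branches on authority, both paths reaching a server event that hands off to BP_GameMode.
; Destruction spawns a BP_Collectable and leaves the GameState player list (last-player check is empty); scene remove/return events toggle visibility, attack and movement.
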(event `self.ReceiveBeginPlay`
  (bind _asw_health_bar (cast `/Game/uIO/State/w_HealthBar` (`WidgetComponent.GetUserWidgetObject` (`self.HpBar`)))
    (:`then`
      (`/Game/uIO/State/w_HealthBar.init` _asw_health_bar self))
    (:`CastFailed`
      (`KismetSystemLibrary.PrintString` "w_HealthBar类型不对"))))

(event `self.ReceiveAnyDamage`
  (params (Damage :type "Float (single-precision)") (DamageType :type "DamageType Object Reference") (InstigatedBy :type "Controller Object Reference") (DamageCauser :type "Actor Object Reference"))
  (`/Game/uIO/State/BPC_State.modifyState` (`self.BPC_State`) "NewEnumerator0" (`KismetMathLibrary.FTrunc` (* -1 Damage))))

(event `Attack`
  (`/Engine/EditorBlueprintResources/ActorMacros.Switch Has Authority`
    (:`Authority`
      (`self.Server_Attack`))
    (:`Remote`
      (`self.Client_Attack`))))

(event `Server_Attack`
  (bind _asbp_game_mode (cast `/Game/uIO/Core/Bp_GameMode` (`GameplayStatics.GetGameMode`)))
  (`/Game/uIO/Core/Bp_GameMode.Attack` _asbp_game_mode self))

(event `Client_Attack`
  (`self.Server_Attack`))

(event `LookAt`
  (params (Target :type "Vector Structure (by ref)"))
  (bind (_returnvalue_roll _returnvalue_pitch _returnvalue_yaw) (`KismetMathLibrary.BreakRotator` (`KismetMathLibrary.FindLookAtRotation` (`self.K2_GetActorLocation`) Target)))
  (`SceneComponent.K2_SetWorldRotation` (`self.Sprite`) (`KismetMathLibrary.MakeRotator` 270.0 0.0 (+ _returnvalue_yaw 90.0)) false false))

(event `self.ReceiveDestroyed`
  (`|SpawnActorFromClass` "/Game/uIO/Collectable/BP_Collectable.BP_Collectable_C" (`self.GetTransform`) "Undefined" "OverrideRootScale" null self null)
  (bind _asbp_game_state (cast `/Game/uIO/Core/BP_GameState` (`GameplayStatics.GetGameState`)))
  (bind _playerlist (`/Game/uIO/Core/BP_GameState.PlayerList` _asbp_game_state))
  (`KismetArrayLibrary.Array_RemoveItem` _playerlist self)
  (if (== (`KismetArrayLibrary.Array_Length` _playerlist) 1)
    _))

(event `/Game/uIO/Core/BPI_Entity.OnRemoveFromScene`
  (`self.SetActorHiddenInGame` true)
  (set `self.canAttack` false)
  (set `self.canMove` false))

(event `/Game/uIO/Core/BPI_Entity.OnReturnToScene`
  (`self.SetActorHiddenInGame` false)
  (set `self.canAttack` true)
  (set `self.canMove` true))

(fn `UserConstructionScript`)