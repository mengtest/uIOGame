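; Player controller for a top-down style character that moves on world axes and aims at the mouse cursor.
; It creates the W_Main widget on BeginPlay and caches the possessed BP_PlayerCharacter, printing a debug message on success or failure.
; Movement and attack inputs are forwarded to that character.
; Every tick it passes the hit location of a Visibility trace under the cursor to the character's LookAt.
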(event `self.ReceiveBeginPlay`
  (bind _returnvalue (`|CreateWidget` "/Game/uIO/Maps/W_Main.W_Main_C"))
  (`UserWidget.AddToViewport` _returnvalue 0))

(event `InputAction|attack`
  (params (Key :type "Key Structure"))
  (bind _playercharacter (`self.PlayerCharacter`))
  (:`Pressed`
    (`/Engine/EditorBlueprintResources/StandardMacros.IsValid` _playercharacter
      (:`Is Valid`
        (`/Game/uIO/Character/BP_CharacterBase.Attack` _playercharacter)))))

(event `self.ReceiveTick`
  (params (DeltaSeconds :type "Float (single-precision)"))
  (bind _playercharacter (`self.PlayerCharacter`))
  (`/Engine/EditorBlueprintResources/StandardMacros.IsValid` _playercharacter
    (:`Is Valid`
      (`/Game/uIO/Character/BP_CharacterBase.LookAt` _playercharacter (`.Location` (`GameplayStatics.BreakHitResult` (`self.GetHitResultUnderCursorByChannel` (`GameplayStatics.GetPlayerController` 0) "TraceTypeQuery1" true)))))))

(event `InputAxis|MoveRight`
  (params (AxisValue :type "Float (single-precision)"))
  (bind _playercharacter (`self.PlayerCharacter`))
  (if (!= AxisValue 0.0)
    (`/Engine/EditorBlueprintResources/StandardMacros.IsValid` _playercharacter
      (:`Is Valid`
        (`Pawn.AddMovementInput` _playercharacter (0.0 1.0 0.0) AxisValue false)))))

(event `InputAxis|MoveForward`
  (params (AxisValue :type "Float (single-precision)"))
  (bind _playercharacter (`self.PlayerCharacter`))
  (if (!= AxisValue 0.0)
    (`/Engine/EditorBlueprintResources/StandardMacros.IsValid` _playercharacter
      (:`Is Valid`
        (`Pawn.AddMovementInput` _playercharacter (1.0 0.0 0.0) AxisValue false)))))

(event `self.ReceivePossess`
  (params (PossessedPawn :type "Pawn Object Reference"))
  (bind _asbp_player_character (cast `/Game/uIO/Character/BP_PlayerCharacter` PossessedPawn)
    (:`then`
      (bind _output_get (set `self.PlayerCharacter` _asbp_player_character))
      (`KismetSystemLibrary.PrintString` (`KismetStringLibrary.Concat_StrStr` "OnPossess" (`KismetSystemLibrary.GetObjectName` _output_get))))
    (:`CastFailed`
      (`KismetSystemLibrary.PrintString` "PlayerController不是BP"))))

(fn `UserConstructionScript`)