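; BP_Block is a destructible block actor that shrinks as bullets hit it.
; An overlapping BP_Bullet is destroyed and the block applies fixed damage to itself, while any other overlap prints a debug string.
; AnyDamage lowers Hp within zero to MaxHp, sets the root's uniform world scale from the health ratio plus a small offset, and destroys the block at zero.
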(event `self.ReceiveActorBeginOverlap`
  (params (OtherActor :type "Actor Object Reference"))
  (bind _asbp_bullet (cast `/Game/uIO/Bullet/BP_Bullet` OtherActor)
    (:`then`
      (`self.K2_DestroyActor` _asbp_bullet)
      (`GameplayStatics.ApplyDamage` self 10.0))
    (:`CastFailed`
      (`KismetSystemLibrary.PrintString` "Hello"))))

(event `self.ReceiveAnyDamage`
  (params (Damage :type "Float (single-precision)") (DamageType :type "DamageType Object Reference") (InstigatedBy :type "Controller Object Reference") (DamageCauser :type "Actor Object Reference"))
  (bind _maxhp (`self.MaxHp`))
  (bind _output_get (set `self.Hp` (`KismetMathLibrary.Clamp` (- (`self.Hp`) (`KismetMathLibrary.FTrunc` Damage)) 0 _maxhp)))
  (bind _returnvalue (+ (/ (`KismetMathLibrary.Conv_IntToDouble` _output_get) (`KismetMathLibrary.Conv_IntToDouble` _maxhp)) 0.2))
  (`SceneComponent.SetWorldScale3D` (`self.DefaultSceneRoot`) (`KismetMathLibrary.MakeVector` _returnvalue _returnvalue _returnvalue))
  (if (== (`self.Hp`) 0)
    (`self.K2_DestroyActor`)))

(fn `UserConstructionScript`)