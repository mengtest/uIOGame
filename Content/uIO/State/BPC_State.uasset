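; BPC_State is a component that stores and updates bounded integer states in a States map.
; GetState looks up an SState struct by key, and SetState adds or overwrites an entry.
; ModifyState adds a delta to a state's Current value, clamps it between that state's Min and Max, and writes the struct back through SetState.
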(fn `getState`
  (params (Key :type "/Game/uIO/State/EState Enum (by ref)" :default "EState_MAX"))
  (returns (Value :type "/Game/uIO/State/SState Structure"))
  (return (`BlueprintMapLibrary.Map_Find` (`self.States`) Key)))

(fn `modifyState`
  (params (State :type "/Game/uIO/State/EState Enum" :default "EState_MAX") (by :type Integer))
  (bind _value (`self.getState` State))
  (bind (_min _max _current) (break `/Game/uIO/State/SState` _value))
  (bind _structout (setmembers `/Game/uIO/State/SState` :`StructRef` _value :`current` (`KismetMathLibrary.Clamp` (+ _current by) _min _max)))
  (`self.setState` State _structout)
  (return))

(fn `setState`
  (params (StateID :type "/Game/uIO/State/EState Enum (by ref)" :default "EState_MAX") (StateInfo :type "/Game/uIO/State/SState Structure (by ref)"))
  (`BlueprintMapLibrary.Map_Add` (`self.States`) StateID StateInfo)
  (return))